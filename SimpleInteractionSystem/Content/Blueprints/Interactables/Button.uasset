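; Interactable button Blueprint that changes its cube's color to show whether it is activated or deactivated.
; BeginPlay creates a dynamic material, sets its emissive strength and applies the starting color from the Interact component's StartActive flag.
; The component's interact and reset delegates drive later color changes through shared logic.
; A key-fetching handler copies HeldKeys from the first Mech_CharacterBP, but its binding is left unconnected.
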(event Custom|Reset%20Status
  (params (Status :type Boolean))
  ;[1 1 1] Change the buttons color to represent status
  (if Status
    (Rendering|Material|SetVectorParameterValue (Variables|Default|GetButtonMat) "Color" (Variables|Default|GetActivated%20Color) :!class /Script/Engine.MaterialInstanceDynamic)
    (else
      (Rendering|Material|SetVectorParameterValue (Variables|Default|GetButtonMat) "Color" (Variables|Default|GetDeactivated%20Color) :!class /Script/Engine.MaterialInstanceDynamic))))

(event Custom|GrabKeys
  (params (Status :type Boolean))
  ;[1 1 1] Simply using an array of ints to hold keys for now, change the actor to your character and plug this up to use keys
  (bind _outactors (Actor|GetAllActorsOfClass "/Game/Blueprints/Mech_CharacterBP.Mech_CharacterBP_C"))
  (Variables|/Script/PuzzleTombGame.InteractComponent|SetcurKeys (Variables|Default|GetInteract) (Variables|/Script/ALSV4_CPP.ALSBaseCharacter|GetheldKeys (Utilities|Array|Get(acopy) _outactors))))

(event Custom|InteractedWith
  (params (Status :type Boolean))
  ;[1 1 1] Change the buttons color to represent status
  (if Status
    (Rendering|Material|SetVectorParameterValue (Variables|Default|GetButtonMat) "Color" (Variables|Default|GetActivated%20Color) :!class /Script/Engine.MaterialInstanceDynamic)
    (else
      (Rendering|Material|SetVectorParameterValue (Variables|Default|GetButtonMat) "Color" (Variables|Default|GetDeactivated%20Color) :!class /Script/Engine.MaterialInstanceDynamic))))

(event EventBeginPlay
  (bind _interact (Variables|Default|GetInteract))
  (Utilities|FlowControl|Sequence
    (:then_0
      ;[1 1 1] Binding the main interaction delegates
      (EventDispatchers|BindEventtoOnInteract _interact (delegate Custom|InteractedWith))
      (EventDispatchers|BindEventtoOnReset _interact (delegate Custom|Reset%20Status))
      ;[1 1 1] Creating Dynamic material
      (bind _returnvalue (Rendering|Material|CreateDynamicMaterialInstance (Variables|Default|GetCube) 0 0 "None" :!class /Script/Engine.PrimitiveComponent))
      (bind _output_get (Variables|Default|SetButtonMat _returnvalue))
      (Rendering|Material|SetScalarParameterValue _output_get "Emissive Color Division" (Variables|Default|GetEmssiveStrength) :!class /Script/Engine.MaterialInstanceDynamic)
      (if (Variables|/Script/PuzzleTombGame.InteractComponent|GetstartActive (Variables|Default|GetInteract))
        (Rendering|Material|SetVectorParameterValue (Variables|Default|GetButtonMat) "Color" (Variables|Default|GetActivated%20Color) :!class /Script/Engine.MaterialInstanceDynamic)
        (else
          (Rendering|Material|SetVectorParameterValue (Variables|Default|GetButtonMat) "Color" (Variables|Default|GetDeactivated%20Color) :!class /Script/Engine.MaterialInstanceDynamic))))))

(fn ConstructionScript)