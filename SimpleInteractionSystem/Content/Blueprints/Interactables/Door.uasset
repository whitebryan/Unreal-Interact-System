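; Interactable sliding double door that toggles between open and closed.
; On BeginPlay it binds a flip-flop event to the InteractableComponent's toggle, which calls OpenDoor or CloseDoor based on the Open flag.
; A single timeline slides the left and right panels apart along relative X in opposite directions, playing to open and reversing to close.
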(event Custom|DoorFlipFlop
  ;[1 1 1] Delegate Setup
  (if (Variables|Default|GetOpen)
    (CallFunction|CloseDoor)
    (else
      (CallFunction|OpenDoor))))

(event Custom|CloseDoor
  (bind _leftdoor (Variables|Default|GetLeftDoor))
  (bind _rightdoor (Variables|Default|GetRightDoor))
  (bind _returnvalue (Transformation|GetRelativeTransform _leftdoor))
  (bind _returnvalue_2 (Transformation|GetRelativeTransform _rightdoor))
  ;[1 1 1] Open door timeline
  (Variables|Default|SetOpen false)
  (Variables|Default|SetDirFloat -1.0)
  (bind _xchange (Timeline|Timeline_0 Reverse)
    (:Update
      (Transformation|SetRelativeLocation (Variables|Default|GetRightDoor) (Math|Vector|MakeVector (+ (* _xchange 145.0) 7e+01) (.y (.location _returnvalue_2)) (.z (.location _returnvalue_2))) false false)
      (Transformation|SetRelativeLocation (Variables|Default|GetLeftDoor) (Math|Vector|MakeVector (+ (* _xchange -145.0) -7e+01) (.y (.location _returnvalue)) (.z (.location _returnvalue))) false false))))

(event Custom|OpenDoor
  (bind _leftdoor (Variables|Default|GetLeftDoor))
  (bind _rightdoor (Variables|Default|GetRightDoor))
  (bind _returnvalue (Transformation|GetRelativeTransform _leftdoor))
  (bind _returnvalue_2 (Transformation|GetRelativeTransform _rightdoor))
  ;[1 1 1] Open door timeline
  (Variables|Default|SetOpen true)
  (Variables|Default|SetDirFloat 1.0)
  (bind _xchange (Timeline|Timeline_0 Play)
    (:Update
      (Transformation|SetRelativeLocation (Variables|Default|GetRightDoor) (Math|Vector|MakeVector (+ (* _xchange 145.0) 7e+01) (.y (.location _returnvalue_2)) (.z (.location _returnvalue_2))) false false)
      (Transformation|SetRelativeLocation (Variables|Default|GetLeftDoor) (Math|Vector|MakeVector (+ (* _xchange -145.0) -7e+01) (.y (.location _returnvalue)) (.z (.location _returnvalue))) false false))))

(event EventBeginPlay
  ;[1 1 1] Delegate Setup
  (EventDispatchers|BindEventtoToggle (Variables|Default|GetInteractableComponent) (delegate Custom|DoorFlipFlop)))

(fn ConstructionScript)