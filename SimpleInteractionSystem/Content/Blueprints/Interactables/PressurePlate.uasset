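; Pressure plate interactable that activates when enough actors overlap its trigger box and deactivates when the count drops below the threshold.
; Overlap begin and end events compare the actor count, less one, against ActorsToActivate, with a Status flag preventing repeat triggers.
; Each state change calls Interact, tints the plate's emissive dynamic material red or white, and plays or reverses a timeline that lowers or raises the plate.
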(event OnComponentBeginOverlap(Box)
  (params (OverlappedComponent :type Primitive%20Component%20Object%20Reference) (OtherActor :type Actor%20Object%20Reference) (OtherComp :type Primitive%20Component%20Object%20Reference) (OtherBodyIndex :type Integer) (bFromSweep :type Boolean) (SweepResult :type Hit%20Result%20Structure%20%28by%20ref%29))
  ;[1 1 1] Detect and activate plate when at least one actor on it
  (if (and (>= (- (Utilities|Array|Length (Collision|GetOverlappingActors (Variables|Default|GetBox) "/Script/Engine.Actor" :!class /Script/Engine.PrimitiveComponent)) 1) (Variables|Default|GetActorsToActivate)) (not (Variables|Default|GetStatus)))
    (Variables|Default|SetStatus true)
    (Class|InteractInterface|Interact (Variables|Default|GetInteract))
    (CallFunction|MovePlate true)))

(event OnComponentEndOverlap(Box)
  (params (OverlappedComponent :type Primitive%20Component%20Object%20Reference) (OtherActor :type Actor%20Object%20Reference) (OtherComp :type Primitive%20Component%20Object%20Reference) (OtherBodyIndex :type Integer))
  ;[1 1 1] Detect when there is no longer any actors on the plate
  (if (and (< (- (Utilities|Array|Length (Collision|GetOverlappingActors (Variables|Default|GetBox) "/Script/Engine.Actor" :!class /Script/Engine.PrimitiveComponent)) 1) (Variables|Default|GetActorsToActivate)) (Variables|Default|GetStatus))
    (Variables|Default|SetStatus false)
    (Class|InteractInterface|Interact (Variables|Default|GetInteract))
    (CallFunction|MovePlate false)))

(event Custom|MovePlate
  (params (Status :type Boolean))
  (bind _plate (Variables|Default|GetPlate))
  (bind _platematerial (Variables|Default|GetPlateMaterial))
  (bind _returnvalue (Transformation|GetRelativeTransform _plate))
  ;[1 1 1] Move the plate up/down timeline
  (if Status
    (Rendering|Material|SetVectorParameterValue _platematerial "Color" "(R=1.000000,G=0.161458,B=0.161458,A=1.000000)" :!class /Script/Engine.MaterialInstanceDynamic)
    (bind _zchange (Timeline|PlateMovement Play)
      (:Update
        (Transformation|SetRelativeLocation _plate (Math|Vector|MakeVector (.x (.location _returnvalue)) (.y (.location _returnvalue)) (+ (* _zchange -5.0) 6.55528)) false false)))
    (else
      (Rendering|Material|SetVectorParameterValue _platematerial "Color" "(R=1.000000,G=1.000000,B=1.000000,A=1.000000)" :!class /Script/Engine.MaterialInstanceDynamic)
      (Timeline|PlateMovement Reverse))))

(event EventBeginPlay
  (bind _returnvalue (Rendering|Material|CreateDynamicMaterialInstance (Variables|Default|GetPlate) 0 0 "None" :!class /Script/Engine.PrimitiveComponent))
  (bind _output_get (Variables|Default|SetPlateMaterial _returnvalue))
  (Rendering|Material|SetVectorParameterValue _output_get "Color" "(R=1.000000,G=1.000000,B=1.000000,A=1.000000)" :!class /Script/Engine.MaterialInstanceDynamic)
  (Rendering|Material|SetScalarParameterValue _output_get "Emissive Color Division" (Variables|Default|GetEmissiveStrength) :!class /Script/Engine.MaterialInstanceDynamic))

(fn ConstructionScript)